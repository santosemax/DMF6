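; BP_DummyEnemy is a simple stationary test enemy that fires projectiles and can be killed.
; From BeginPlay it loops on a Delay, spawning BP_ky_fireBall every few seconds at a fixed world-X offset with the actor's rotation.
; AnyDamage updates the HealthBarAboveHead widget with Health minus Damage, then destroys the actor if the Health component reads zero or below.
; It never writes Health itself, and an AddToViewport node is left unconnected.
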(event EventBeginPlay
  (Utilities|FlowControl|Sequence
    (:then_0
      (Game|SpawnActorfromClass "/Game/FXVarietyPack/Blueprints/BP_ky_fireBall.BP_ky_fireBall_C" (Math|Transform|MakeTransform (- (Transformation|GetActorLocation) "200.000000, 0, 0") (Transformation|GetActorRotation) "1,1,1") "Undefined" 0 0 :!label _label)
      (Utilities|FlowControl|Delay 3.0)
      (goto _label))))

(event Game|Damage|EventAnyDamage
  (params (Damage :type Float%20%28single-precision%29) (DamageType :type Damage%20Type%20Object%20Reference) (InstigatedBy :type Controller%20Object%20Reference) (DamageCauser :type Actor%20Object%20Reference))
  (bind _health (Variables|Default|GetHealth))
  (bind _ashealth_bar_above_head (Utilities|Casting|CastToHealthBarAboveHead (UserInterface|GetWidget (Variables|Default|GetHealthBar))))
  (Default|UpdateHealth _ashealth_bar_above_head (- (Variables|/Script/Movecpp.HealthComponent|Gethealth _health) Damage) (Variables|/Script/Movecpp.HealthComponent|GetmaxHealth _health))
  (if (<= (Variables|/Script/Movecpp.HealthComponent|Gethealth (Variables|Default|GetHealth)) 0.0)
    (Actor|DestroyActor)))

(fn ConstructionScript)