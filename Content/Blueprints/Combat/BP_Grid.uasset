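; BP_Grid is a tile grid actor that draws configurable lines and a highlight for a selected tile.
; The construction script builds both as procedural mesh quads via CreateLine, using dynamic M_Grid materials for colour and opacity; the highlight is one tile-thick line.
; SetSelectedTile moves the highlight to the world position from TileToGridLocation.
; LocationToTile and TileValid? are stubs, and TileToGridLocation always reports valid.
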(event EventBeginPlay)

(event Collision|EventActorBeginOverlap
  (params (OtherActor :type Actor%20Object%20Reference)))

(event EventTick
  (params (DeltaSeconds :type Float%20%28single-precision%29)))

(fn ConstructionScript
  (bind _tilesize (Variables|Constants|GetTileSize))
  (bind _returnvalue (/ _tilesize 2.0))
  (bind _materialintstance (Private|CreateMaterialInstance (Variables|Appearence|GetLineColour) (Variables|Appearence|GetLineOpacity)))
  (LocalVariables|SetLineMaterialInstance _materialintstance)
  (bind _materialintstance_2 (Private|CreateMaterialInstance (Variables|Appearence|GetSelectionColour) (Variables|Appearence|GetSelectionOpacity)))
  (LocalVariables|SetLineSelectionInstance _materialintstance_2)
  (Utilities|FlowControl|Sequence
    (:then_0
      ;[1 1 1] Drawing the Row Lines
      (for _index (range 0 (Variables|Constants|GetNumRows))
        (LocalVariables|SetlineStart (* _index (Variables|Constants|GetTileSize)))
        (LocalVariables|SetlineEnd (Private|GridWidth))
        (Private|CreateLine (Math|Vector|MakeVector (LocalVariables|GetlineStart) 0.0 0.0) (Math|Vector|MakeVector (LocalVariables|GetlineStart) (LocalVariables|GetlineEnd) 0.0) (Variables|Appearence|GetLineThickness) (LocalVariables|GetLineVertices) (LocalVariables|GetLine%20Triangles))))
    (:then_1
      ;[1 1 1] Drawing the Vertical Lines
      (for _index_2 (range 0 (Variables|Constants|GetNumCols))
        (LocalVariables|SetlineStart (* _index_2 (Variables|Constants|GetTileSize)))
        (LocalVariables|SetlineEnd (Private|GridHeight))
        (Private|CreateLine (Math|Vector|MakeVector 0.0 (LocalVariables|GetlineStart) 0.0) (Math|Vector|MakeVector (LocalVariables|GetlineEnd) (LocalVariables|GetlineStart) 0.0) (Variables|Appearence|GetLineThickness) (LocalVariables|GetLineVertices) (LocalVariables|GetLine%20Triangles))))
    (:then_2
      ;[1 1 1] Create Procedural Mesh For Lines
      (Class|ProceduralMeshComponent|CreateMeshSectionLinearColor (Variables|Default|GetProceduralMesh) 0 (LocalVariables|GetLineVertices) (LocalVariables|GetLine%20Triangles) 0 0 0 0 0 0 0 false)
      (Rendering|Material|SetMaterial (Variables|Default|GetProceduralMesh) 0 (LocalVariables|GetLineMaterialInstance)))
    (:then_3
      ;[1 1 1] Create Selection Geometry
      (Private|CreateLine (Math|Vector|MakeVector 0.0 _returnvalue 0.0) (Math|Vector|MakeVector _tilesize _returnvalue 0.0) (Variables|Constants|GetTileSize) (LocalVariables|GetSelection%20Vertices) (LocalVariables|GetSelection%20Triangles))
      (Class|ProceduralMeshComponent|CreateMeshSectionLinearColor (Variables|Default|GetSelectionMesh) 0 (LocalVariables|GetSelection%20Vertices) (LocalVariables|GetSelection%20Triangles) 0 0 0 0 0 0 0 false)
      (Rendering|Material|SetMaterial (Variables|Default|GetSelectionMesh) 0 (LocalVariables|GetLineSelectionInstance)))))

(fn CreateLine
  (params (Start :type Vector) (End :type Vector) (Thickness :type Float%20%28single-precision%29) (Vertices :type Array%20of%20Vectors) (Triangles :type Array%20of%20Integers))
  (bind _returnvalue (Utilities|Array|Length Vertices))
  (Utilities|FlowControl|Sequence
    (:then_0
      (LocalVariables|SethalfThickness (/ Thickness 2.0))
      (LocalVariables|SetThickness%20Direction (Math|Vector|CrossProduct (Math|Vector|Normalize (- End Start)) "0, 0,1.000000")))
    (:then_1
      (Utilities|Array|AppendArray Triangles (Utilities|Array|MakeArray (+ _returnvalue 2) (+ _returnvalue 1) (+ _returnvalue 0) (+ _returnvalue 2) (+ _returnvalue 3) (+ _returnvalue 1)))
      (Utilities|Array|AppendArray Vertices (Utilities|Array|MakeArray (+ Start (* (LocalVariables|GetThickness%20Direction) (LocalVariables|GethalfThickness))) (+ End (* (LocalVariables|GetThickness%20Direction) (LocalVariables|GethalfThickness))) (- Start (* (LocalVariables|GetThickness%20Direction) (LocalVariables|GethalfThickness))) (- End (* (LocalVariables|GetThickness%20Direction) (LocalVariables|GethalfThickness))))))))

(fn GridWidth
  (return (* (Variables|Constants|GetNumCols) (Variables|Constants|GetTileSize))))

(fn CreateMaterialInstance
  (params (Color :type Linear%20Color%20Structure) (Opacity :type Float%20%28single-precision%29))
  (bind _returnvalue (Rendering|Material|CreateDynamicMaterialInstance "/Game/Blueprints/Combat/M_Grid.M_Grid" "None" "None" :!class /Script/Engine.KismetMaterialLibrary))
  (Rendering|Material|SetVectorParameterValue _returnvalue "Color" Color :!class /Script/Engine.MaterialInstanceDynamic)
  (Rendering|Material|SetScalarParameterValue _returnvalue "Opacity" Opacity :!class /Script/Engine.MaterialInstanceDynamic)
  (return _returnvalue))

(fn GridHeight
  (return (* (Variables|Constants|GetNumRows) (Variables|Constants|GetTileSize))))

(fn LocationtoTile
  (params (Location :type Vector))
  (return 0 0))

(fn TiletoGridLocation
  (params (Row :type Integer) (Col :type Integer) (Center? :type Boolean))
  (bind _returnvalue (Transformation|GetActorLocation))
  (bind _tilesize (Variables|Constants|GetTileSize))
  (bind _returnvalue_2 (/ _tilesize 2.0))
  (bind _returnvalue_3 (select Center? _returnvalue_2 0.0))
  (return true (Math|Vector2D|MakeVector2D (+ (+ (* Row (Variables|Constants|GetTileSize)) (.x _returnvalue)) _returnvalue_3) (+ (+ (.y _returnvalue) (* Col (Variables|Constants|GetTileSize))) _returnvalue_3))))

(fn SetSelectedTile
  (params (Row :type Integer) (Col :type Integer))
  (bind (_valid_ _gridlocation) (CallFunction|TiletoGridLocation Row Col false))
  (if _valid_
    (Rendering|SetVisibility (Variables|Default|GetSelectionMesh) true false)
    (Transformation|SetWorldLocation (Variables|Default|GetSelectionMesh) (Math|Vector|MakeVector (.X (Math|Vector2D|BreakVector2D _gridlocation)) (.Y (Math|Vector2D|BreakVector2D _gridlocation)) (.z (Transformation|GetActorLocation))) false false)
    (else
      (Rendering|SetVisibility (Variables|Default|GetSelectionMesh) false false))))