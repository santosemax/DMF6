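; Player character blueprint for a tile-grid game, with test input for tile selection and fireball attacks.
; BeginPlay gets the Grid from BP_AnimaGameModeBase and adds the HUD widget to the viewport.
; Arrow keys step the tracked row and column to set the selected tile, while R spawns a fireball at a fixed world X offset.
; Damage pushes reduced health to the HUD without storing it on the Health variable.
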(event EventBeginPlay
  (Utilities|FlowControl|Sequence
    (:then_0
      (bind _asbp_anima_game_mode_base (Utilities|Casting|CastToBP_AnimaGameModeBase (Game|GetGameMode)))
      (bind _grid (Default|GetGrid _asbp_anima_game_mode_base))
      (Variables|Default|SetGrid _grid))
    (:then_1
      (bind _returnvalue (UserInterface|CreateWidget "/Game/Combat/HUD_Widget.HUD_Widget_C"))
      (bind _output_get (Variables|Default|SetHUD _returnvalue))
      (UserInterface|Viewport|AddtoViewport _output_get 0))))

(event Game|Damage|EventAnyDamage
  (params (Damage :type Float%20%28single-precision%29) (DamageType :type Damage%20Type%20Object%20Reference) (InstigatedBy :type Controller%20Object%20Reference) (DamageCauser :type Actor%20Object%20Reference))
  (bind _health (Variables|Default|GetHealth))
  ;[1 1 1] Testing sutff just to see how things feel
  (Default|UpdateHealth (Variables|Default|GetHUD) (- (Variables|/Script/Movecpp.HealthComponent|Gethealth _health) Damage) (Variables|/Script/Movecpp.HealthComponent|GetmaxHealth _health)))

(event Input|KeyboardEvents|Up
  (params (Key :type Key%20Structure :default "None"))
  ;[1 1 1] Testing sutff just to see how things feel
  (:Pressed
    (Development|PrintString "Movin up" true true "(R=0.000000,G=0.000000,B=0.000000,A=1.000000)")
    (Default|SetSelectedTile (Variables|Default|GetGrid) (+ (Variables|Default|GetcurrRow) 1) (Variables|Default|GetcurrCol))
    (Variables|Default|SetcurrRow (+ (Variables|Default|GetcurrRow) 1))))

(event Input|KeyboardEvents|Right
  (params (Key :type Key%20Structure :default "None"))
  ;[1 1 1] Testing sutff just to see how things feel
  (:Pressed
    (Development|PrintString "Right" true true "(R=0.000000,G=0.000000,B=0.000000,A=1.000000)")
    (Default|SetSelectedTile (Variables|Default|GetGrid) (Variables|Default|GetcurrRow) (+ (Variables|Default|GetcurrCol) 1))
    (Variables|Default|SetcurrCol (+ (Variables|Default|GetcurrCol) 1))))

(event Input|KeyboardEvents|Down
  (params (Key :type Key%20Structure :default "None"))
  ;[1 1 1] Testing sutff just to see how things feel
  (:Pressed
    (Development|PrintString "Down" true true "(R=0.000000,G=0.000000,B=0.000000,A=1.000000)")
    (Default|SetSelectedTile (Variables|Default|GetGrid) (+ (Variables|Default|GetcurrRow) -1) (Variables|Default|GetcurrCol))
    (Variables|Default|SetcurrRow (+ (Variables|Default|GetcurrRow) -1))))

(event Input|KeyboardEvents|Left
  (params (Key :type Key%20Structure :default "None"))
  ;[1 1 1] Testing sutff just to see how things feel
  (:Pressed
    (Development|PrintString "Left" true true "(R=0.000000,G=0.000000,B=0.000000,A=1.000000)")
    (Default|SetSelectedTile (Variables|Default|GetGrid) (Variables|Default|GetcurrRow) (+ (Variables|Default|GetcurrCol) -1))
    (Variables|Default|SetcurrCol (+ (Variables|Default|GetcurrCol) -1))))

(event Input|KeyboardEvents|R
  (params (Key :type Key%20Structure :default "None"))
  ;[1 1 1] Testing sutff just to see how things feel
  (:Pressed
    (Development|PrintString "Fire")
    (Game|SpawnActorfromClass "/Game/FXVarietyPack/Blueprints/BP_ky_fireBall.BP_ky_fireBall_C" (Math|Transform|MakeTransform (+ (Transformation|GetActorLocation) "250.000000,0.000000,0.000000") "0, 0, 0" "1,1,1") "Undefined" 0 0)))

(fn ConstructionScript)

(fn EventPromptTrigger)